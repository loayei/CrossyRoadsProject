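; Water floor chunk that spawns three floor sections, landing nodes and optional flowers or moving logs.
; With logs enabled, it pre-fills the row on BeginPlay, then Tick spawns more off one side on a timer.
; Random log length sets spacing and spawn delay, while a per-row random speed bonus shortens the delay.
; Tick also runs the chunk's destruction check, and destruction removes its flowers.
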(event `self.ReceiveBeginPlay`
  (bind (_tranform_left _tranform_mid _tranform_right) (`self.Calculate Floor Transform`))
  (bind _returnvalue (`|SpawnActorFromClass` "/Game/Assets/Blueprints/BP_Floor.BP_Floor_C" _tranform_left "Undefined" "OverrideRootScale" null 2 false self null))
  (set `self.Left Floor` _returnvalue)
  (bind _returnvalue_2 (`|SpawnActorFromClass` "/Game/Assets/Blueprints/BP_Floor.BP_Floor_C" _tranform_mid "Undefined" "OverrideRootScale" null 2 true self null))
  (set `self.Center Floor` _returnvalue_2)
  (bind _returnvalue_3 (`|SpawnActorFromClass` "/Game/Assets/Blueprints/BP_Floor.BP_Floor_C" _tranform_right "Undefined" "OverrideRootScale" null 2 false self null))
  (set `self.Right Floor` _returnvalue_3)
  (`self.Construct Landing Nodes`)
  (if (`self.Create Logs`)
    (`self.Construct Initial Logs`)))

(event `self.ReceiveTick`
  (params (DeltaSeconds :type "Float (single-precision)"))
  (if (`self.Create Logs`)
    (`self.Construct Log Attempt` DeltaSeconds))
  (`self.Check IF Destroy Floor Chunk`))

(event `self.ReceiveDestroyed`
  (for _array_element (`self.Flowers`)
    (`self.K2_DestroyActor` _array_element)))

(fn `Add Extra Log Speed Random`
  (set `self.Extra Log Speed Center` (`KismetMathLibrary.RandomFloatInRange` 0.0 200.0)))

(fn `Calculate Log Creation Offset Next`
  (returns (`Random X Position` :type "Float (double-precision)"))
  (`/Engine/EditorBlueprintResources/StandardMacros.IsValid` (`self.Current Log Created`)
    (:`Is Valid`
      (switch `int` (`/Game/Assets/Blueprints/BP_Log.Length` (`self.Current Log Created`))
        (:`1`
          (return (`KismetMathLibrary.RandomFloatInRange` 400.0 500.0)))
        (:`2`
          (return (`KismetMathLibrary.RandomFloatInRange` 600.0 700.0)))
        (:`3`
          (return (`KismetMathLibrary.RandomFloatInRange` 800.0 900.0)))))
    (:`Is Not Valid`
      (return (`KismetMathLibrary.RandomFloatInRange` 0.0 100.0)))))

(fn `Construct Flower`
  (params (`Current X` :type "Float (double-precision)"))
  (bind (_returnvalue_x _returnvalue_y _returnvalue_z) (`KismetMathLibrary.BreakVector` (`self.K2_GetActorLocation`)))
  (if (== `Current X` -1.0)
    (bind _returnvalue (`|SpawnActorFromClass` "/Game/Assets/Blueprints/BP_Flower.BP_Flower_C" (`KismetMathLibrary.MakeTransform` (`KismetMathLibrary.MakeVector` `Current X` _returnvalue_y (- _returnvalue_z 30.0))) "Undefined" "OverrideRootScale" null null))
    (`KismetArrayLibrary.Array_Add` (`self.Flowers`) _returnvalue)))

(fn `Construct Flowersss`
  (bind _current_clear_column_pos_x3 (`self.Current Clear Column Pos X3`))
  (if (>= (`self.Number Of Flowers To Create`) 1)
    (`self.Construct Flower` (`self.Current Clear Column Pos X1`))
    (if (>= (`self.Number Of Flowers To Create`) 2)
      (if (not (== (`self.Current Clear Column Pos X1`) (`self.Current Clear Column Pos X2`)))
        (`self.Construct Flower` (`self.Current Clear Column Pos X2`))
        (if (>= (`self.Number Of Flowers To Create`) 3)
          (if (not (or (== _current_clear_column_pos_x3 (`self.Current Clear Column Pos X1`)) (== (`self.Current Clear Column Pos X2`) _current_clear_column_pos_x3)))
            (`self.Construct Flower` (`self.Current Clear Column Pos X3`))))))))

(fn `Construct Initial Logs`
  (locals (`Log Create X Position` :type "Float (double-precision)"))
  (if (`self.Create Logs Left`)
    (set `local.Log Create X Position` -900.0)
    (while (< (`local.Log Create X Position`) 900.0)
      (bind _random_x_position (`self.Calculate Log Creation Offset Next`))
      (bind _output_get (set `local.Log Create X Position` (+ _random_x_position (`local.Log Create X Position`))))
      (`self.Construct Log` _output_get))
    (else
      (set `local.Log Create X Position` 900.0)
      (while (> (`local.Log Create X Position`) -900.0)
        (bind _random_x_position_2 (`self.Calculate Log Creation Offset Next`))
        (bind _output_get_2 (set `local.Log Create X Position` (- (`local.Log Create X Position`) _random_x_position_2)))
        (`self.Construct Log` _output_get_2)))))

(fn `Construct Landing Nodes`
  (set `self.Current Z Position For Landing Node` -60.0)
  (for _ (range 9)
    (`self.Construct Landing Node (Floor Chunk)` true))
  (if (`self.Create Flower`)
    (`self.Construct Flowersss`)))

(fn `Construct Log`
  (params (`Location X` :type "Float (double-precision)"))
  (returns (`Return Log` :type "/Game/Assets/Blueprints/BP_Log Object Reference"))
  (bind (_returnvalue_x _returnvalue_y _returnvalue_z) (`KismetMathLibrary.BreakVector` (`self.K2_GetActorLocation`)))
  (bind _returnvalue (`|SpawnActorFromClass` "/Game/Assets/Blueprints/BP_Log.BP_Log_C" (`KismetMathLibrary.MakeTransform` (`KismetMathLibrary.MakeVector` `Location X` _returnvalue_y _returnvalue_z)) "Undefined" "OverrideRootScale" null (`KismetMathLibrary.RandomIntegerInRange` 1 3) (not (`self.Create Logs Left`)) (`self.Extra Log Speed Center`) null))
  (bind _output_get (set `self.Current Log Created` _returnvalue))
  (return _output_get))

(fn `Construct Log Attempt`
  (params (`Delta TIme` :type "Float (double-precision)"))
  (bind _returnvalue (/ (`self.Extra Log Speed Center`) 400.0))
  (bind _output_get (set `self.Current Create Log Time` (+ `Delta TIme` (`self.Current Create Log Time`))))
  (if (>= _output_get (`self.MAX Create Log Time`))
    (if (`self.Create Logs Left`)
      (`self.Construct Log` -2800.0)
      (else
        (`self.Construct Log` 2800.0)))
    (set `self.Current Create Log Time` 0.0)
    (switch `int` (`/Game/Assets/Blueprints/BP_Log.Length` (`self.Current Log Created`))
      (:`1`
        (set `self.MAX Create Log Time` (- (`KismetMathLibrary.RandomFloatInRange` 1.25 1.5) _returnvalue)))
      (:`2`
        (set `self.MAX Create Log Time` (- (`KismetMathLibrary.RandomFloatInRange` 1.5 1.75) _returnvalue)))
      (:`3`
        (set `self.MAX Create Log Time` (- (`KismetMathLibrary.RandomFloatInRange` 2.0 2.25) _returnvalue))))))

(fn `UserConstructionScript`
  (if (`self.Create Logs`)
    (set `self.MAX Create Log Time` (`KismetMathLibrary.RandomFloatInRange` 0.0 1.0))
    (`self.Add Extra Log Speed Random`)))