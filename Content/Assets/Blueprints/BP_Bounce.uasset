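; BP_Bounce is an actor that briefly dips vertically when flagged as being jumped on.
; Tick advances a timer while the flag is set; after a start delay, a hard-coded quadratic curve drives a Z offset from the cached height.
; The animation resets 0.2 seconds after the delay, returning the actor to that height.
; Neither the flag's activation nor the height caching happens in these graphs.
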(event `self.ReceiveBeginPlay`
  (set `self.MAX Jumped On Time` (+ (`self.MAX Start Jump Time`) 0.2)))

(event `self.ReceiveTick`
  (params (DeltaSeconds :type "Float (single-precision)"))
  (`self.Bouncing Animation` DeltaSeconds))

(fn `Bouncing Animation`
  (params (`Delta Time` :type "Float (double-precision)"))
  (bind (_returnvalue_x _returnvalue_y) (`KismetMathLibrary.BreakVector` (`self.K2_GetActorLocation`)))
  (if (`self.Is Being Jumped On`)
    (`self.Jumped On Animation` `Delta Time`)
    (`self.K2_SetActorLocation` (`KismetMathLibrary.MakeVector` _returnvalue_x _returnvalue_y (+ (`self.Cashed Z Position`) (`self.Jumped On Z Offset`))))))

(fn `Jumped On Animation`
  (params (`Delta Time` :type "Float (double-precision)"))
  (set `self.Current Jumped On Time` (+ `Delta Time` (`self.Current Jumped On Time`)))
  (if (>= (`self.Current Jumped On Time`) (`self.MAX Start Jump Time`))
    (if (>= (`self.Current Jumped On Time`) (`self.MAX Jumped On Time`))
      (`self.Reset Animation`)
      (else
        (set `self.Jumped On Z Offset` (* (- (`KismetMathLibrary.Square` (- (* (- (`self.Current Jumped On Time`) 0.1) 8.0) 1.0)) 1.0) 20.0))))))

(fn `Reset Animation`
  (set `self.Is Being Jumped On` false)
  (set `self.Jumped On Z Offset` 0.0)
  (set `self.Current Jumped On Time` 0.0))

(fn `UserConstructionScript`)